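; AI character Blueprint that can be damaged, equip items and be stealth-assassinated from behind.
; It equips a starting item, shows its mesh as the held object, and binds stats to a camera-facing health bar.
; Damage plays a random hit reaction and sound, launches it along the player's forward vector, and calls Die at zero health.
; An overlap radius toggles the assassinate prompt; assassination plays a victim montage, with Die's delayed ragdoll as a temporary fix.
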(event OnComponentBeginOverlap(AssassinationRadius)
  (params (OverlappedComponent :type Primitive%20Component%20Object%20Reference) (OtherActor :type Actor%20Object%20Reference) (OtherComp :type Primitive%20Component%20Object%20Reference) (OtherBodyIndex :type Integer) (bFromSweep :type Boolean) (SweepResult :type Hit%20Result%20Structure%20%28by%20ref%29))
  (Utilities|Casting|CastToBP_ThirdPersonCharacter OtherActor)
  (Rendering|SetVisibility (Variables|Default|GetAssassinateWidget) true false))

(event OnComponentEndOverlap(AssassinationRadius)
  (params (OverlappedComponent :type Primitive%20Component%20Object%20Reference) (OtherActor :type Actor%20Object%20Reference) (OtherComp :type Primitive%20Component%20Object%20Reference) (OtherBodyIndex :type Integer))
  (Utilities|Casting|CastToBP_ThirdPersonCharacter OtherActor)
  (Rendering|SetVisibility (Variables|Default|GetAssassinateWidget) false false))

(event Custom|Ragdoll
  (Physics|SetSimulatePhysics (Variables|Character|GetMesh) true))

(event Custom|Die
  (Utilities|FlowControl|Delay 2.5) ; Temp fix for assassination. Should update
  (CallFunction|Ragdoll)
  (Rendering|SetVisibility (Variables|Default|GetHealthBar) false false)
  (Collision|SetCollisionEnabled (Variables|Default|GetCapsuleComponent) "NoCollision")
  (Collision|SetCollisionEnabled (Variables|Default|GetAssassinationRadius) "NoCollision"))

(event Game|Damage|EventAnyDamage
  (params (Damage :type Float%20%28single-precision%29) (DamageType :type Damage%20Type%20Object%20Reference) (InstigatedBy :type Controller%20Object%20Reference) (DamageCauser :type Actor%20Object%20Reference))
  (bind _hit_react_anims (Variables|Default|GetHit%20React%20Anims))
  (bind _returnvalue (Class|CharacterStatsComponent|DecreaseHealth (Variables|Default|GetCharacterStats) Damage))
  (Animation|Montage|PlayMontage (Variables|Character|GetMesh) (Utilities|Array|Get(acopy) _hit_react_anims (Math|Random|RandomIntegerinRange 0 (- (Utilities|Array|Length _hit_react_anims) 1)))
    (:then
      (Audio|PlaySoundatLocation "/Game/Audio/Grunts/SC_Death.SC_Death" (Transformation|GetActorLocation) "0, 0, 0" 1.0 (Math|Random|RandomFloatinRange 0.85 1.2) 0.0 "/Game/Audio/SA_Character.SA_Character" 0 0 0)
      (Character|LaunchCharacter (* (Transformation|GetActorForwardVector (Game|GetPlayerCharacter 0)) 7e+02) false false)
      (if _returnvalue
        (CallFunction|Die)))))

(event EventTick
  (params (DeltaSeconds :type Float%20%28single-precision%29))
  (bind _healthbar (Variables|Default|GetHealthBar))
  (|CallParentFunction 0.0)
  (Transformation|SetWorldRotation _healthbar (Math|Rotator|FindLookatRotation (Transformation|GetWorldLocation _healthbar) (Transformation|GetWorldLocation (Variables|/Script/Engine.PlayerCameraManager|GetTransformComponent (Game|GetPlayerCameraManager 0)))) false false))

(event EventBeginPlay
  (|CallParentFunction)
  (bind _aswb_floating_health_bar (Utilities|Casting|CastToWB_FloatingHealthBar (UserInterface|GetWidget (Variables|Default|GetHealthBar))))
  (Default|SetStatsComponent _aswb_floating_health_bar (Variables|Default|GetCharacterStats))
  (bind _returnvalue (Class|InventoryInterface|AddInventoryItem (Variables|Default|GetStartingEquipedItem)))
  (Class|RPGTutorialCharacter|EquipItem _returnvalue))

(event EventOnItemEquipped
  (params (Item :type Inventory%20Item%20Object%20Reference))
  (bind _itemdefinition (Variables|/Script/RPG_Tutorial.InventoryItem|GetItemDefinition Item))
  (Utilities|IsValid Item
    (:Is%20Valid
      (Utilities|IsValid _itemdefinition
        (:Is%20Valid
          (Components|StaticMesh|SetStaticMesh (Variables|Default|GetHeldObject) (Variables|/Script/RPG_Tutorial.ItemDefinition|GetMesh _itemdefinition)))))))

(fn ConstructionScript)

(fn GetEquipedItemMesh
  (return (Variables|Default|GetHeldObject)))

(fn AttemptStealthBackAssassinate
  (Animation|PlayAnimMontage "/Game/Characters/RPG_Character/Animations/Assassinations/Paired_Knife_Stealth_KidneyAndNeck_Vic_Montage.Paired_Knife_Stealth_KidneyAndNeck_Vic_Montage" 1.0 "None")
  (CallFunction|Die)
  (Rendering|SetVisibility (Variables|Default|GetAssassinateWidget) false false)
  (return (Transformation|GetWorldLocation (Variables|Default|GetAssassin%20REF)) (Transformation|GetActorRotation)))