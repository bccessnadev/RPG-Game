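; Attack component for the RPG character that runs melee combo attacks and their hit detection.
; Attack input, gated to equipped melee weapons, feeds combo objects that start, continue or cancel chains.
; A looping timer sphere-traces between weapon sockets, applying damage, camera shake, sound and blood to "Attackable" actors, throttled by a delayed DoOnce.
; A temporary foot-socket trace handles kick hits.
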(event Custom|Sword%20Attack%20Combo
  ;[1 0.821 0.115] Combo continue
  (for _array_element (Variables|Default|GetActiveCombos)
    (Class|ComboAttack|TryStartNextAttack _array_element)))

(event Custom|Start%20Sword%20Trace
  ;[0.3444 1 0.5153] Sword Trace
  (bind _returnvalue (Utilities|Time|SetTimerbyEvent (delegate Custom|Sword%20Trace%20Loop) 0.01 true))
  (Variables|Default|SetSword%20Trace%20Loop%20Handle _returnvalue))

(event Custom|Sword%20Trace%20Loop
  (bind _character (Variables|Default|GetCharacter))
  (bind _returnvalue (Class|RPGTutorialCharacter|GetEquipedItemMesh _character))
  ;[0.3444 1 0.5153] Sword Trace
  (Utilities|IsValid _returnvalue
    (:Is%20Valid
      (bind (_outhit _returnvalue_2) (Collision|SphereTraceByChannel (Transformation|GetSocketLocation _returnvalue "HitTraceStart") (Transformation|GetSocketLocation _returnvalue "HitTraceEnd") 12.0 "TraceTypeQuery1" false 0 "None"))
      (if _returnvalue_2
        (if (Actor|ActorHasTag (.HitActor (Collision|BreakHitResult _outhit)) "Attackable")
          (Utilities|FlowControl|DoOnce false :!label _label
            (:Completed
              (Game|Damage|ApplyDamage (.HitActor (Collision|BreakHitResult _outhit)) 1e+01 0 (Components|GetOwner))
              (Camera|PlayWorldCameraShake "/Game/GameplaySystems/AttackSytems/BP_AttackCameraShake.BP_AttackCameraShake_C" (.Location (Collision|BreakHitResult _outhit)) 0.0 2e+03)
              (Audio|PlaySoundatLocation "/Game/Audio/SwordHits/MS_SwordHit.MS_SwordHit" (.Location (Collision|BreakHitResult _outhit)) "0, 0, 0" 1.0 1.0 0.0 0 0 0 0)
              (Effects|SpawnEmitteratLocation "/Game/VFX/Particles/Blood/P_Blood_Splat_Cone.P_Blood_Splat_Cone" (.Location (Collision|BreakHitResult _outhit)) (Math|Rotator|MakeRotfromXY (.Normal (Collision|BreakHitResult _outhit)) (.Normal (Collision|BreakHitResult _outhit))) "0.500000,0.500000,0.500000" true "AutoRelease")
              (Utilities|FlowControl|Delay 0.5)
              (goto _label Reset))))))))

(event Custom|End%20Sword%20Trace%20Loop
  ;[0.3444 1 0.5153] Sword Trace
  (Utilities|Time|ClearandInvalidateTimerbyHandle (Variables|Default|GetSword%20Trace%20Loop%20Handle)))

(event Custom|Kick%20Trace
  (bind _owner_mesh (Variables|Default|GetOwner%20Mesh))
  (bind _returnvalue (Transformation|GetSocketLocation _owner_mesh "foot_r_Socket"))
  ;[0.3444 1 0.5153] Kick Trace
  (bind (_outhit _returnvalue_2) (Collision|SphereTraceByChannel _returnvalue _returnvalue 25.0 "TraceTypeQuery1" false 0 "None"))
  (if _returnvalue_2
    (if (Actor|ActorHasTag (.HitActor (Collision|BreakHitResult _outhit)) "Attackable")
      (Game|Damage|ApplyDamage (.HitActor (Collision|BreakHitResult _outhit)) 1e+01 0 (Components|GetOwner))
      (Camera|PlayWorldCameraShake "/Game/GameplaySystems/AttackSytems/BP_AttackCameraShake.BP_AttackCameraShake_C" (.Location (Collision|BreakHitResult _outhit)) 0.0 2e+03))))

(event Custom|Stop%20Sword%20Combo
  ;[1 0.3723 0.05754] Stop combo
  (for _array_element (Variables|Default|GetActiveCombos)
    (Class|ComboAttack|CancelCombo _array_element)
    (Utilities|Array|RemoveIndex (Variables|Default|GetActiveCombos))))

(event Custom|Handle%20Attack%20Input
  (params (Input%20Action :type Input%20Action%20Object%20Reference))
  (bind _activecombos (Variables|Default|GetActiveCombos))
  ;[1 0.821 0.115] Combo logic
  (if (Utilities|Array|IsEmpty _activecombos)
    ;;[0.2825 1 0.3984] Try to start a new combo
    (for _array_element (Variables|Default|GetComboAttacks) :!label _label
      (bind _returnvalue (Class|ComboAttack|TryAttack _array_element Input%20Action))
      (if _returnvalue
        (Utilities|Array|Add (Variables|Default|GetActiveCombos) _array_element)))
    (else
      ;;[0.1898 0.8902 1] Try continuing active combos
      (for _array_element_2 _activecombos
        (Class|ComboAttack|TryAttack _array_element_2 Input%20Action))
      (if (Utilities|Array|IsEmpty _activecombos) ; If all of the active combos fail, \ntry to start a new one
        (goto _label)))))

(event Input|EnhancedActionEvents|EnhancedInputActionIA_Attack
  (params (ActionValue :type Boolean) (ElapsedSeconds :type Float%20%28double-precision%29) (TriggeredSeconds :type Float%20%28double-precision%29) (InputAction :type Input%20Action%20Object%20Reference :default "/Game/Input/Actions/IA_Attack.IA_Attack"))
  ;[0.1812 0.1779 0.162] Attack input
  (:Started
    (if (CallFunction|CanAttack)
      (CallFunction|HandleAttackInput InputAction))))

(event EventBeginPlay
  ;[0.04067 0.5729 0.04335] Begin Play
  (bind _asrpg_tutorial_character (Utilities|Casting|CastToRPG_TutorialCharacter (Components|GetOwner)))
  (bind _output_get (Variables|Default|SetCharacter _asrpg_tutorial_character))
  (Variables|Default|SetOwner%20Mesh (Variables|/Script/Engine.Character|GetMesh _output_get))
  (bind _returnvalue (Class|ComboAttack|CreateComboAttack (Variables|Default|GetBasicSwordComboAttacks) _output_get))
  (Utilities|Array|Add (Variables|Default|GetComboAttacks) _returnvalue))

(fn CanAttack
  (bind _character (Variables|Default|GetCharacter))
  (bind _returnvalue (Class|RPGTutorialCharacter|GetEquippedItem _character))
  (bind _itemdefinition (Variables|/Script/RPG_Tutorial.InventoryItem|GetItemDefinition _returnvalue))
  (Utilities|IsValid _character
    (:Is%20Valid
      (Utilities|IsValid _returnvalue
        (:Is%20Valid
          (Utilities|IsValid _itemdefinition
            (:Is%20Valid
              (return (and (Variables|Default|GetbCanAttack) (Class|GameplayStatics|ObjectIsA _itemdefinition "/Script/RPG_Tutorial.MeleeWeaponItemDefinition"))))))))))