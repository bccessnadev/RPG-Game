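; BP_InteractPrompt is an actor that shows a widget prompt on the current interactable target with that target's interaction message.
; On BeginPlay it caches the text block from its WP_InteractPrompt widget.
; SetInteractActor either snaps the prompt onto a valid target, shows it and enables tick, or hides, detaches and stops ticking.
; While ticking, it refreshes the text each frame from the target's GetInteractTextMessage.
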(event Custom|Set%20Interact%20Actor
  (params (New%20Interact%20Actor :type Actor%20Object%20Reference))
  ;[1 0.821 0.115] Set interact actor
  (bind _output_get (Variables|Default|SetTargetActor New%20Interact%20Actor))
  (Utilities|IsValid _output_get
    (:Is%20Valid
      (Transformation|AttachActorToActor (Variables|Default|GetTargetActor) "None" "SnapToTarget" "SnapToTarget" "SnapToTarget" true)
      (Rendering|SetVisibility (Variables|Default|GetInteractPrompt) true false)
      (Actor|Tick|SetActorTickEnabled true))
    (:Is%20Not%20Valid
      (Rendering|SetVisibility (Variables|Default|GetInteractPrompt) false false)
      (Transformation|DetachFromActor "KeepRelative" "KeepRelative" "KeepRelative")
      (Actor|Tick|SetActorTickEnabled false))))

(event EventTick
  (params (DeltaSeconds :type Float%20%28single-precision%29))
  ;[0.2901 1 0.7347] Update Interact text on tick
  (bind _targetactor (Variables|Default|GetTargetActor)
    (:then
      (bind _interact_text (Variables|Default|GetInteract%20Text)
        (:then
          (bind _returnvalue (Class|InteractInterface|GetInteractText(Message) _targetactor))
          (Rendering|Components|TextRender|SetText _interact_text (Utilities|Text|ToText(String) _returnvalue)))
        (:else)))
    (:else)))

(event EventBeginPlay
  ;[0.04067 0.5729 0.04335] Begin play
  (bind _aswp_interact_prompt (Utilities|Casting|CastToWP_InteractPrompt (UserInterface|GetWidget (Variables|Default|GetInteractPrompt))))
  (bind _output_get (Variables|Default|SetInteractWidget _aswp_interact_prompt))
  (Variables|Default|SetInteract%20Text (Variables|/Game/UI/WP_InteractPrompt.WP_InteractPrompt_C|GetInteractText _output_get)))

(fn ConstructionScript)