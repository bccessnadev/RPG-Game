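; Equipment system component for the third-person character that handles showing and hiding the equipment menu.
; The IA_EquipmentMenu input flips MenuOpened to either create the WB_Equipment widget or remove it, switching mouse cursor and input mode to match.
; While the menu shows, it disables character movement and clears CanAttack on the attack system component, then restores walking and attacking on close.
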(event Input|EnhancedActionEvents|EnhancedInputActionIA_EquipmentMenu
  (params (ActionValue :type Boolean) (ElapsedSeconds :type Float%20%28double-precision%29) (TriggeredSeconds :type Float%20%28double-precision%29) (InputAction :type Input%20Action%20Object%20Reference :default "/Game/Input/Actions/IA_EquipmentMenu.IA_EquipmentMenu"))
  (bind _returnvalue (Game|GetPlayerController 0))
  (bind _returnvalue_2 (Components|GetOwner))
  (bind _returnvalue_3 (Actor|GetComponentbyClass _returnvalue_2 "/Script/Engine.CharacterMovementComponent"))
  (:Started
    (bind _output_get (Variables|Default|SetbMenuOpened (not (Variables|Default|GetbMenuOpened))))
    (if _output_get
      (bind _menu_widget (Variables|Default|GetMenu%20Widget)
        (:then
          (Widget|RemovefromParent _menu_widget)
          (Variables|Default|SetMenu%20Widget 0)
          (Variables|/Script/Engine.PlayerController|SetbShowMouseCursor _returnvalue false)
          (Input|SetInputModeGameOnly _returnvalue false)
          (Pawn|Components|CharacterMovement|SetMovementMode _returnvalue_3 "MOVE_Walking" 0)
          (bind _as_bp_third_person_character (Variables|Default|GetAs%20BP%20Third%20Person%20Character)
            (:then
              (bind _bpc_attacksystem (Variables|/Game/Characters/RPG_Character/BP_ThirdPersonCharacter.BP_ThirdPersonCharacter_C|GetBPC_AttackSystem _as_bp_third_person_character)
                (:then
                  (Variables|/Game/GameplaySystems/AttackSytems/BPC_AttackSystem.BPC_AttackSystem_C|SetbCanAttack _bpc_attacksystem true))
                (:else)))
            (:else)))
        (:else))
      (else
        (bind _returnvalue_4 (UserInterface|CreateWidget "/Game/GameplaySystems/Equipment/UI/WB_Equipment.WB_Equipment_C"))
        (bind _output_get_2 (Variables|Default|SetMenu%20Widget _returnvalue_4))
        (UserInterface|Viewport|AddtoViewport _output_get_2 0)
        (Variables|/Script/Engine.PlayerController|SetbShowMouseCursor _returnvalue true)
        (Input|SetInputModeGameandUI _returnvalue (Variables|Default|GetMenu%20Widget) "DoNotLock" true false)
        (Pawn|Components|CharacterMovement|SetMovementMode _returnvalue_3 "MOVE_None" 0)
        (bind _as_bp_third_person_character_2 (Variables|Default|GetAs%20BP%20Third%20Person%20Character)
          (:then
            (bind _bpc_attacksystem_2 (Variables|/Game/Characters/RPG_Character/BP_ThirdPersonCharacter.BP_ThirdPersonCharacter_C|GetBPC_AttackSystem _as_bp_third_person_character_2)
              (:then
                (Variables|/Game/GameplaySystems/AttackSytems/BPC_AttackSystem.BPC_AttackSystem_C|SetbCanAttack _bpc_attacksystem_2 false))
              (:else)))
          (:else))))))

(event EventBeginPlay
  (bind _asbp_third_person_character (Utilities|Casting|CastToBP_ThirdPersonCharacter (Components|GetOwner)))
  (Variables|Default|SetAs%20BP%20Third%20Person%20Character _asbp_third_person_character))