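; Player stats component that tracks health, stamina, XP and level for its owning actor.
; Increase and decrease functions clamp current values, with decreases reporting depletion, and fire update delegates passing the new values.
; Tick regenerates stamina while the owner's velocity is at or below a threshold.
; Reaching max XP levels up once, carrying over excess, raising the next requirement by level and playing a sound.
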(event Custom|Update%20Stamina
  (params (Delta%20Seconds :type Float%20%28double-precision%29))
  (bind _returnvalue (Components|GetOwner))
  (Utilities|IsValid _returnvalue
    (:Is%20Valid
      (if (<= (Math|Vector|VectorLength (Transformation|GetVelocity _returnvalue)) (Variables|Stamina|GetStaminaRegenMinVelocity))
        (Stamina|IncreaseStamina (* (Variables|Stamina|GetStaminaRegenRate) Delta%20Seconds))))))

(event EventTick
  (params (DeltaSeconds :type Float%20%28single-precision%29))
  (CallFunction|UpdateStamina DeltaSeconds))

(fn DecreaseHealth
  (params (Damage :type Float%20%28double-precision%29))
  (bind _output_get (Variables|Health|SetCurrent%20Health (Math|Float|Max(Float) (- (Variables|Health|GetCurrent%20Health) Damage) 0.0)))
  (Health|OnHealthUpdated)
  (return (== _output_get 0.0)))

(fn IncreaseMaxHealth
  (params (Max%20Health%20Increase :type Float%20%28double-precision%29))
  (Variables|Health|SetMax%20Health (+ Max%20Health%20Increase (Variables|Health|GetMax%20Health)))
  (Health|OnHealthUpdated))

(fn DecreaseStamina
  (params (Stamina%20Decrease :type Float%20%28double-precision%29))
  (bind _output_get (Variables|Stamina|SetCurrent%20Stamina (Math|Float|Max(Float) (- (Variables|Stamina|GetCurrent%20Stamina) Stamina%20Decrease) 0.0)))
  (Stamina|OnStaminaUpdated)
  (return (== _output_get 0.0)))

(fn IncreaseMaxStamina
  (params (Max%20Stamina%20Increase :type Float%20%28double-precision%29))
  (Variables|Stamina|SetMax%20Stamina (+ Max%20Stamina%20Increase (Variables|Stamina|GetMax%20Stamina)))
  (Stamina|OnStaminaUpdated))

(fn IncreaseStamina
  (params (Stamina%20Increase :type Float%20%28double-precision%29))
  (Variables|Stamina|SetCurrent%20Stamina (Math|Float|Min(Float) (+ Stamina%20Increase (Variables|Stamina|GetCurrent%20Stamina)) (Variables|Stamina|GetMax%20Stamina)))
  (Stamina|OnStaminaUpdated))

(fn IncreaseHealth
  (params (Health%20Increase :type Float%20%28double-precision%29))
  (Variables|Health|SetCurrent%20Health (Math|Float|Min(Float) (+ Health%20Increase (Variables|Health|GetCurrent%20Health)) (Variables|Health|GetMax%20Health)))
  (Health|OnHealthUpdated))

(fn OnHealthUpdated
  (Default|CallOnHealthUpdatedDelegate (Variables|Health|GetCurrent%20Health) (Variables|Health|GetMax%20Health)))

(fn OnStaminaUpdated
  (Default|CallOnStaminaUpdatedDelegate (Variables|Stamina|GetCurrent%20Stamina) (Variables|Stamina|GetMax%20Stamina)))

(fn IncreaseXP
  (params (XP%20Increase :type Float%20%28double-precision%29))
  (bind _output_get (Variables|XP|SetXP (+ XP%20Increase (Variables|XP|GetXP))))
  (if (>= _output_get (Variables|XP|GetMax%20XP))
    (XP|IncreaseLevel 1)
    (else
      (XP|OnXPUpdated))))

(fn IncreaseLevel
  (params (Level%20Increase :type Integer))
  (Variables|XP|SetLevel (+ Level%20Increase (Variables|XP|GetLevel)))
  (Variables|XP|SetXP (- (Variables|XP|GetXP) (Variables|XP|GetMax%20XP)))
  (Variables|XP|SetMax%20XP (+ (Variables|XP|GetMax%20XP) (* (Variables|XP|GetLevel) 150)))
  (XP|OnXPUpdated)
  (Audio|PlaySound2D "/Game/Audio/UI/SW_LevelUp.SW_LevelUp" 1.0 1.0 0.0 0 0))

(fn OnXPUpdated
  (Default|CallOnXPUpdatedDelegate (Variables|XP|GetXP) (Variables|XP|GetMax%20XP) (Variables|XP|GetLevel)))